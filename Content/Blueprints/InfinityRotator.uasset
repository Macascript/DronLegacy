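; InfinityRotator is a component that endlessly rotates its owning actor at a fixed interval.
; On BeginPlay it caches the owner's root component and initial rotation, then starts a looping timer at UpdateFrecuency instead of using Tick.
; Each DoRotate call combines RotationStep with the root's current world rotation and prints a debug string.
; The stored initial rotation is not read in these graphs.
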(event EventBeginPlay
  (bind _returnvalue (Components|GetOwner))
  (bind _rootcomponent (Variables|/Script/Engine.Actor|GetRootComponent _returnvalue))
  (Variables|Default|SetRoot _rootcomponent)
  (Variables|Default|SetinitialRotation (Transformation|GetWorldRotation _rootcomponent))
  (Utilities|Time|SetTimerbyFunctionName 0 "DoRotate" (Variables|Default|GetupdateFrecuency) true))

(event EventTick
  (params (DeltaSeconds :type Float%20%28single-precision%29)))

(fn DoRotate
  (Transformation|SetWorldRotation (Variables|Default|GetRoot) (Math|Rotator|CombineRotators (Transformation|GetWorldRotation (Variables|Default|GetRoot)) (Variables|Default|GetrotationStep)) false false)
  (Development|PrintString "Llamado"))