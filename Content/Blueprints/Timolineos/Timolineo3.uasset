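; Timolineo3 is an actor that continuously moves up and down between its spawn location and a point 1000 units above it.
; On BeginPlay it stores both endpoints and plays the StartToEnd timeline, whose Lerp track blends the actor's location between them.
; Each time the timeline finishes, it prints a debug string and a FlipFlop alternates between reversing and replaying it, creating an endless ping-pong motion.
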(event EventBeginPlay
  (bind _returnvalue (Transformation|GetActorLocation))
  (Variables|Default|SetStartLocation _returnvalue)
  (Variables|Default|SetEndLocation (+ _returnvalue "0.000000,0,1000.000000"))
  (bind _lerp (Timeline|startToEnd Play)
    (:Update
      (Transformation|SetActorLocation (Math|Vector|Lerp(Vector) (Variables|Default|GetStartLocation) (Variables|Default|GetEndLocation) _lerp) false false))
    (:Finished
      (Development|PrintString "Hello")
      (Utilities|FlowControl|FlipFlop
        (:A
          (Timeline|startToEnd ReverseFromEnd))
        (:B
          (Timeline|startToEnd PlayFromStart))))))

(event Collision|EventActorBeginOverlap
  (params (OtherActor :type Actor%20Object%20Reference)))

(event EventTick
  (params (DeltaSeconds :type Float%20%28single-precision%29)))

(fn ConstructionScript)