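; Player controller that switches control between the character Krombopulos, a ship (Nave) and Troni.
; E leaves the ship by possessing Krombopulos and teleporting him to NaveEnterPoint, or boards it when he is within MinDistance of that point.
; CambiarPersonaje toggles IsKrom outside the ship without changing possession.
; When both IsNave and IsKrom are false, Tick forwards movement axes to Troni.
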(event EventBeginPlay)

(event EventTick
  (params (DeltaSeconds :type Float%20%28single-precision%29))
  (if (Math|Boolean|NORBoolean (Variables|Default|GetisNave) (Variables|Default|GetisKrom))
    (Default|SetAxis (Variables|Default|GetTroni) (Input|AxisValues|GetMoveRight/Left) (Input|AxisValues|GetMoveForward/Backward) (Input|AxisValues|GetMoveUp/Down))))

(event Input|ActionEvents|InputActionCambiarPersonaje
  (params (Key :type Key%20Structure :default "None"))
  (:Pressed
    (if (not (Variables|Default|GetisNave))
      (Variables|Default|SetisKrom (not (Variables|Default|GetisKrom))))))

(event Input|KeyboardEvents|E
  (params (Key :type Key%20Structure :default "None"))
  (bind _krombopulos (Variables|Default|GetKrombopulos))
  (bind _krombopulos_2 (Variables|Default|GetKrombopulos))
  (bind _mindistance (Variables|Default|GetMinDistance))
  (bind _naveenterpoint (Variables|Default|GetNaveEnterPoint))
  (bind _naveenterpoint_2 (Variables|Default|GetNaveEnterPoint))
  (bind _returnvalue (Transformation|GetWorldLocation _naveenterpoint_2))
  (bind _returnvalue_2 (Transformation|GetActorLocation _krombopulos_2))
  (bind _returnvalue_3 (Math|Vector|Distance(Vector) _returnvalue_2 _returnvalue))
  (bind _returnvalue_4 (< _returnvalue_3 _mindistance))
  (:Pressed
    (if (Variables|Default|GetisNave)
      (Pawn|Possess _krombopulos)
      (Development|PrintString (Utilities|GetDisplayName _naveenterpoint))
      (Transformation|SetActorLocation _krombopulos (Transformation|GetWorldLocation _naveenterpoint) false true)
      (Variables|Default|SetisNave false)
      (elif _returnvalue_4
        (Development|PrintString (Utilities|String|ToString(Boolean) _returnvalue_4))
        (Pawn|Possess (Variables|Default|GetNave))
        (Variables|Default|SetisNave true)))))

(fn ConstructionScript)