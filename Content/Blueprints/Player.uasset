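; Player Blueprint that moves the actor from the Horizontal and Vertical input axes.
; Each Tick it scales the right and forward vectors by axis values, Speed and delta time, then applies their sum through AddActorLocalOffset without sweep.
; The offset is applied in local space although both direction vectors are world-space.
; The axis events, unconnected AddMovementInput nodes, construction script and NewFunction0 do nothing.
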(event EventBeginPlay)

(event Collision|EventActorBeginOverlap
  (params (OtherActor :type Actor%20Object%20Reference)))

(event EventTick
  (params (DeltaSeconds :type Float%20%28single-precision%29))
  (bind _speed (Variables|Default|GetSpeed))
  (Transformation|AddActorLocalOffset (* DeltaSeconds (+ (* (Transformation|GetActorRightVector) (Input|AxisValues|GetHorizontal) _speed) (* _speed (Transformation|GetActorForwardVector) (Input|AxisValues|GetVertical)))) false false))

(event Input|AxisEvents|InputAxisHorizontal
  (params (AxisValue :type Float%20%28single-precision%29))
  ;[1 1 1] USELESS
)

(event Input|AxisEvents|InputAxisVertical
  (params (AxisValue :type Float%20%28single-precision%29))
  ;[1 1 1] USELESS
)

(fn ConstructionScript)

(fn NewFunction0)